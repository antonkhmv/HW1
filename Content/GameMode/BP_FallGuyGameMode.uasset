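; Game mode for a Fall Guys-style obstacle game that holds the current level's parameters and manages boost effects.
; On BeginPlay it loads LevelParams from DT_LevelParams, using the level stored in GI_Store_Level as the row name.
; Speed boosts halve rotation, obstacle and spike speeds, while wall boosts enable overlapping on every BP_Hurdle.
; Per-boost counters handle stacking, applying each effect on the first pickup and reverting it on the last removal.
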(event Custom|RemoveSpeedBoost
  ;[1 1 1] Handle boosts
  (bind _result (Math|Integer|DecrementInt (Variables|Default|GetSpeedBoostCount))
    (:%20%20
      (if (== _result 0)
        (Variables|Default|SetLevelParams (Utilities|Struct|MakeST_LevelParams (.level (Variables|Default|GetLevelParams)) (* (.rotationspeed (Variables|Default|GetLevelParams)) 2.0) (* (.obstaclespeed (Variables|Default|GetLevelParams)) 2.0) (* (.spikesspeed (Variables|Default|GetLevelParams)) 2.0) (.hurdletype (Variables|Default|GetLevelParams)) (.n_platforms (Variables|Default|GetLevelParams))))))))

(event Custom|RemoveWallBoost
  ;[1 1 1] Handle boosts
  (bind _result (Math|Integer|DecrementInt (Variables|Default|GetWallBoostCount))
    (:%20%20
      (if (== _result 0)
        (bind _outactors (Actor|GetAllActorsOfClass "/Game/Blueprints/Platforms/Hurdle/BP_Hurdle.BP_Hurdle_C"))
        (for _array_element _outactors
          (Default|DisableOverlapping _array_element))))))

(event Custom|PickedSpeedBoost
  ;[1 1 1] Handle boosts
  (bind _result (Math|Integer|IncrementInt (Variables|Default|GetSpeedBoostCount))
    (:%20%20
      (if (== _result 1)
        (Variables|Default|SetLevelParams (Utilities|Struct|MakeST_LevelParams (.level (Variables|Default|GetLevelParams)) (* (.rotationspeed (Variables|Default|GetLevelParams)) 0.5) (* (.obstaclespeed (Variables|Default|GetLevelParams)) 0.5) (* (.spikesspeed (Variables|Default|GetLevelParams)) 0.5) (.hurdletype (Variables|Default|GetLevelParams)) (.n_platforms (Variables|Default|GetLevelParams))))))))

(event Custom|PickedWallBoost
  ;[1 1 1] Handle boosts
  (bind _result (Math|Integer|IncrementInt (Variables|Default|GetWallBoostCount))
    (:%20%20
      (if (== _result 1)
        (bind _outactors (Actor|GetAllActorsOfClass "/Game/Blueprints/Platforms/Hurdle/BP_Hurdle.BP_Hurdle_C"))
        (for _array_element _outactors
          (Default|EnableOverlapping _array_element))))))

(event EventBeginPlay
  ;[1 1 1] get params
  (bind _asgi_store_level (Utilities|Casting|CastToGI_Store_Level (Game|GetGameInstance)))
  (bind _returnvalue (Utilities|GetDataTableRow "/Game/GameMode/DT_LevelParams.DT_LevelParams" (Utilities|String|StringToName (Utilities|String|ToString(Integer) (Variables|/Game/GameMode/GI_Store_Level.GI_Store_Level_C|GetLevel _asgi_store_level))))
    (:then
      (Variables|Default|SetLevelParams _returnvalue)
      (Variables|Default|SetSpeedBoostCount 0)
      (Variables|Default|SetWallBoostCount 0))))

(fn ConstructionScript)