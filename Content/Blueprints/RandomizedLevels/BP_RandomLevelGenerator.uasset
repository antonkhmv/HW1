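; Level generator actor that builds a random path of platforms from streamed level instances, starting beside the origin cell.
; GenerateLevel walks a grid left, right or forward, restricting turns by the last two directions to keep the path one platform wide, then caps it with a final level.
; SetRandomPlatform instances a random level at each cell and may spawn one speed or wall boost, using conditional probability to preserve each boost's intended chance.
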(event Custom|Generate%20Level
  ;[1 1 1] (Cell 0, 0 is the begining)
  (Variables|Default|SetDirection "NewEnumerator2")
  (Variables|Default|SetprevDirection "NewEnumerator2")
  (Variables|Default|SetY 1)
  (Variables|Default|SetX 0)
  ;[1 1 1] While loop
  (while (< (Variables|Default|GetI) (Variables|Default|GetN))
    (CallFunction|SetRandomPlatform (Variables|Default|GetLevel_names) true)
    ;[1 1 1] Chosing a random direction
    (Variables|Default|Settemp (Variables|Default|GetDirection))
    (Variables|Default|SetDirection (Utilities|Array|Get(acopy) (Utilities|Select :Index (select (Utilities|Enum|Equal(Enum) (Variables|Default|GetprevDirection) "NewEnumerator2") (Variables|Default|GetDirection) (Variables|Default|GetprevDirection)) :NewEnumerator0 (Utilities|Array|MakeArray "NewEnumerator0" "NewEnumerator2") :NewEnumerator1 (Utilities|Array|MakeArray "NewEnumerator1" "NewEnumerator2") :NewEnumerator2 (Utilities|Array|MakeArray "NewEnumerator1" "NewEnumerator2" "NewEnumerator0")) (Math|Random|RandomInteger (Utilities|Array|Length (Utilities|Select :Index (select (Utilities|Enum|Equal(Enum) (Variables|Default|GetprevDirection) "NewEnumerator2") (Variables|Default|GetDirection) (Variables|Default|GetprevDirection)) :NewEnumerator0 (Utilities|Array|MakeArray "NewEnumerator0" "NewEnumerator2") :NewEnumerator1 (Utilities|Array|MakeArray "NewEnumerator1" "NewEnumerator2") :NewEnumerator2 (Utilities|Array|MakeArray "NewEnumerator1" "NewEnumerator2" "NewEnumerator0"))))))
    (Variables|Default|SetprevDirection (Variables|Default|Gettemp))
    ;;[1 1 1] update the coordinates according to the current direction
    (Utilities|FlowControl|Sequence
      (:then_0
        (switch Utilities|FlowControl|Switch|SwitchonDirection (Variables|Default|GetDirection)
          (:NewEnumerator0
            (Math|Integer|DecrementInt (Variables|Default|GetX)))
          (:NewEnumerator1
            (Math|Integer|IncrementInt (Variables|Default|GetX)))
          (:NewEnumerator2
            (Math|Integer|IncrementInt (Variables|Default|GetY)))))
      (:then_1
        (Math|Integer|IncrementInt (Variables|Default|GetI)))))
  ;[1 1 1] Last platform
  (CallFunction|SetRandomPlatform (Utilities|Array|MakeArray (Variables|Default|GetLast_Level_Name)) false))

(event Collision|EventActorBeginOverlap
  (params (OtherActor :type Actor%20Object%20Reference)))

(event EventTick
  (params (DeltaSeconds :type Float%20%28single-precision%29)))

(fn ConstructionScript)

(fn SetRandomPlatform
  (params (NamesArray :type Array%20of%20Names) (Generate%20Boosts :type Boolean))
  (bind _y (Variables|Default|GetY))
  (bind _x (Variables|Default|GetX))
  (bind _level_size (Variables|Default|GetLevel_size))
  (bind _level_size_2 (Variables|Default|GetLevel_size))
  (bind _returnvalue (* _x _level_size))
  (bind _returnvalue_2 (* _y _level_size_2))
  (bind _returnvalue_3 (Math|Vector|MakeVector _returnvalue _returnvalue_2 0.0))
  (bind _returnvalue_4 (Math|Transform|MakeTransform _returnvalue_3))
  ;[1 1 1] Pick random platform
  (Utilities|FlowControl|Sequence
    (:then_0
      ;[1 1 1] Add stremaing level
      (bind _returnvalue_5 (Class|LevelStreaming|CreateInstance (Class|GameplayStatics|GetStreamingLevel (Utilities|Array|Get(acopy) NamesArray (Math|Random|RandomIntegerinRange 0 (Utilities|Array|LastIndex NamesArray)))) (Utilities|String|Append (Utilities|String|ToString(Integer) (Variables|Default|GetY)) "" (Utilities|String|ToString(Integer) (Variables|Default|GetX)))))
      (Variables|/Script/Engine.LevelStreaming|SetbShouldBeLoaded _returnvalue_5 true)
      (Variables|/Script/Engine.LevelStreaming|SetbShouldBeVisible _returnvalue_5 true)
      (Variables|/Script/Engine.LevelStreaming|SetLevelTransform _returnvalue_5 _returnvalue_4))
    (:then_1
      (if Generate%20Boosts
        (Utilities|FlowControl|Sequence
          (:then_1
            ;[1 1 1] Add boosts
            (if (< (Math|Random|RandomFloat) (Variables|Default|GetSpeedBoostP))
              (Game|SpawnActorfromClass "/Game/Blueprints/Boosts/BP_BoostSpeed.BP_BoostSpeed_C" _returnvalue_4 "Undefined" 0 0)
              (elif (< (Math|Random|RandomFloat) (/ (Variables|Default|GetWallBoostP) (- 1.0 (Variables|Default|GetSpeedBoostP))))
                (Game|SpawnActorfromClass "/Game/Blueprints/Boosts/BP_BoostWalls.BP_BoostWalls_C" _returnvalue_4 "Undefined" 0 0)))))))))