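; BP_Hammer is an obstacle that slides back and forth and knocks Fall Guy characters away on overlap.
; Tick advances a wrapped phase scaled by the game mode's obstacle speed, moving the hammer sinusoidally along its forward vector within HalfDistance.
; Overlap launches the character along world X or Y, chosen by IsRotated, with cosine-scaled velocity matching the swing's phase.
; IsInverse mirrors both motion and launch direction.
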(event EventBeginPlay
  (Variables|Default|SetLocation (Transformation|GetWorldLocation (Variables|Default|GetHammer)))
  (bind _asbp_fall_guy_game_mode (Utilities|Casting|CastToBP_FallGuyGameMode (Game|GetGameMode)))
  (Variables|Default|Setgamemode _asbp_fall_guy_game_mode))

(event Collision|EventActorBeginOverlap
  (params (OtherActor :type Actor%20Object%20Reference))
  (bind _isinverse (Variables|Default|GetisInverse))
  (bind _returnvalue (select _isinverse -1.0 1.0))
  (bind _asbp_fall_guy_character (Utilities|Casting|CastToBP_FallGuyCharacter OtherActor))
  (bind _returnvalue_2 (CallFunction|GetCos))
  (bind _returnvalue_3 (CallFunction|Lerp _returnvalue_2 1e+03))
  (Character|LaunchCharacter _asbp_fall_guy_character (* (select (Variables|Default|GetisRotated) (Math|Vector|MakeVector 0.0 _returnvalue 0.0) (Math|Vector|MakeVector _returnvalue 0.0 0.0)) _returnvalue_3) true false))

(event EventTick
  (params (DeltaSeconds :type Float%20%28single-precision%29))
  (Variables|Default|SetOffset (Math|Float|%(Float) (+ (* 3.0 DeltaSeconds (.obstaclespeed (Variables|/Game/GameMode/BP_FallGuyGameMode.BP_FallGuyGameMode_C|GetLevelParams (Variables|Default|Getgamemode)))) (Variables|Default|GetOffset)) (* (Math|Trig|GetPI) 2.0)))
  (bind _returnvalue (CallFunction|GetSin))
  (bind _returnvalue_2 (CallFunction|Lerp _returnvalue (Variables|Default|GetHalfDistance)))
  (Transformation|SetWorldLocation (Variables|Default|GetHammer) (+ (* (Math|Vector|GetForwardVector (Math|Rotator|CombineRotators (Transformation|GetWorldRotation (Variables|Default|GetHammer)) "0, 0, 0")) _returnvalue_2) (Variables|Default|GetLocation)) false false))

(fn ConstructionScript)

(fn GetSin
  (return (Math|Trig|Sin(Radians) (* (select (Variables|Default|GetisInverse) -1.0 1.0) (Variables|Default|GetOffset)))))

(fn GetCos
  (return (Math|Trig|Cos(Radians) (Variables|Default|GetOffset))))

(fn Lerp
  (params (A :type Float%20%28single-precision%29) (B :type Float%20%28single-precision%29))
  (return (Math|Float|Lerp (- 0.0 B) B (/ (+ A 1.0) 2.0))))