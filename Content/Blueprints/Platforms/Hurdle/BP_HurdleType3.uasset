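; BP_HurdleType3 is a platform hurdle that can switch between a solid, opaque state and a transparent, passable one.
; The construction script caches the static mesh's original materials.
; MakeTransparent puts M_Transparent on every material slot and disables collision, while MakeOpaque restores the cached materials and sets collision to BlockAll.
; The file does not contain the logic that triggers either event.
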(event EventMakeTransparent
  (Utilities|FlowControl|Sequence
    (:then_0
      (for _index (range 0 (Utilities|Array|LastIndex (Variables|Default|GetMaterials)))
        (Rendering|Material|SetMaterial (Variables|Default|GetStaticMesh) _index "/Game/Materials/M_Transparent.M_Transparent")))
    (:then_1
      (Collision|SetCollisionProfileName (Variables|Default|GetStaticMesh) "NoCollision" true :!class /Script/Engine.PrimitiveComponent))))

(event EventMakeOpaque
  (bind _materials (Variables|Default|GetMaterials))
  (for _index (range 0 (Utilities|Array|LastIndex _materials))
    (Rendering|Material|SetMaterial (Variables|Default|GetStaticMesh) _index (Utilities|Array|Get(acopy) _materials _index))
    (Collision|SetCollisionProfileName (Variables|Default|GetStaticMesh) "BlockAll" true :!class /Script/Engine.PrimitiveComponent)))

(fn ConstructionScript
  (Variables|Default|SetMaterials (Rendering|Material|GetMaterials (Variables|Default|GetStaticMesh))))