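; BP_Hurdle is a platform hurdle wrapper that builds the hurdle variant chosen for the current level.
; On construction, AddHurdle reads HurdleType from BP_FallGuyGameMode's LevelParams and adds one of three child actor components, stored as Hurdle.
; EnableOverlapping and DisableOverlapping forward MakeTransparent and MakeOpaque to that child through BP_Interface_HurdleType.
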(event Custom|DisableOverlapping
  (bind _asbp_interface_hurdle_type (Utilities|Casting|CastToBP_Interface_HurdleType (Variables|/Script/Engine.ChildActorComponent|GetChildActor (Variables|Default|GetHurdle))))
  (Default|MakeOpaque _asbp_interface_hurdle_type))

(event Custom|EnableOverlapping
  (bind _asbp_interface_hurdle_type (Utilities|Casting|CastToBP_Interface_HurdleType (Variables|/Script/Engine.ChildActorComponent|GetChildActor (Variables|Default|GetHurdle))))
  (Default|MakeTransparent _asbp_interface_hurdle_type))

(event EventBeginPlay)

(event Collision|EventActorBeginOverlap
  (params (OtherActor :type Actor%20Object%20Reference)))

(event EventTick
  (params (DeltaSeconds :type Float%20%28single-precision%29)))

(fn ConstructionScript
  (CallFunction|AddHurdle))

(fn AddHurdle
  (bind _asbp_fall_guy_game_mode (Utilities|Casting|CastToBP_FallGuyGameMode (Game|GetGameMode)))
  (switch int (.hurdletype (Variables|/Game/GameMode/BP_FallGuyGameMode.BP_FallGuyGameMode_C|GetLevelParams _asbp_fall_guy_game_mode))
    (:1
      (bind _returnvalue (AddComponent|AddChildActorComponent false))
      (Variables|Default|SetHurdle _returnvalue))
    (:2
      (bind _returnvalue_2 (AddComponent|AddChildActorComponent false))
      (Variables|Default|SetHurdle _returnvalue_2))
    (:3
      (bind _returnvalue_3 (AddComponent|AddChildActorComponent false))
      (Variables|Default|SetHurdle _returnvalue_3))))