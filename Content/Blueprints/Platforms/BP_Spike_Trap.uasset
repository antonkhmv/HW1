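; Spike trap hazard that cycles vertically and calls Death on any BP_FallGuyCharacter that overlaps its spike mesh.
; BeginPlay caches the mesh's start location and the game mode, whose LevelParams spike speed advances a wrapped phase every Tick.
; A sine of that phase, clamped and normalised by Scale, lerps the height between raised and lowered, allowing holds at the extremes.
; IsInverse flips the cycle so traps can alternate.
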(event OnComponentBeginOverlap(SpikeTrap01)
  (params (OverlappedComponent :type Primitive%20Component%20Object%20Reference) (OtherActor :type Actor%20Object%20Reference) (OtherComp :type Primitive%20Component%20Object%20Reference) (OtherBodyIndex :type Integer) (bFromSweep :type Boolean) (SweepResult :type Hit%20Result%20Structure%20%28by%20ref%29))
  (bind _asbp_fall_guy_character (Utilities|Casting|CastToBP_FallGuyCharacter OtherActor))
  (Default|Death _asbp_fall_guy_character))

(event EventBeginPlay
  (Variables|Default|SetLocation (Transformation|GetWorldLocation (Variables|Default|GetSpike%20Trap%2001)))
  (bind _asbp_fall_guy_game_mode (Utilities|Casting|CastToBP_FallGuyGameMode (Game|GetGameMode)))
  (Variables|Default|Setgamemode _asbp_fall_guy_game_mode))

(event Collision|EventActorBeginOverlap
  (params (OtherActor :type Actor%20Object%20Reference)))

(event EventTick
  (params (DeltaSeconds :type Float%20%28single-precision%29))
  (bind _location (Variables|Default|GetLocation))
  (bind _scale (Variables|Default|GetScale))
  (bind _output_get (Variables|Default|SetOffset (Math|Float|%(Float) (+ (* 1.5 DeltaSeconds (.spikesspeed (Variables|/Game/GameMode/BP_FallGuyGameMode.BP_FallGuyGameMode_C|GetLevelParams (Variables|Default|Getgamemode)))) (Variables|Default|GetOffset)) (* (Math|Trig|GetPI) 2.0))))
  (Transformation|SetWorldLocation (Variables|Default|GetSpike%20Trap%2001) (Math|Vector|MakeVector (.x _location) (.y _location) (+ (.z _location) (Math|Float|Lerp 1e+01 -1e+02 (/ (Math|Float|Clamp(Float) (+ (* (Math|Trig|Sin(Radians) _output_get) (select (Variables|Default|GetisInverse) -1.0 1.0)) (/ _scale 2.0)) 0.0 (Variables|Default|GetScale)) _scale)))) false false))

(fn ConstructionScript)