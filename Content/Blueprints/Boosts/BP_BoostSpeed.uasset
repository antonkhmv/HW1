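; Speed boost pickup actor that grants a timed speed boost when a BP_FallGuyCharacter overlaps its box.
; The overlap tells BP_FallGuyGameMode to apply the boost, then destroys the box and coin components so the pickup cannot be collected again.
; The actor stays alive for Duration, then has the game mode remove the boost and destroys itself.
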(event OnComponentBeginOverlap(Box)
  (params (OverlappedComponent :type Primitive%20Component%20Object%20Reference) (OtherActor :type Actor%20Object%20Reference) (OtherComp :type Primitive%20Component%20Object%20Reference) (OtherBodyIndex :type Integer) (bFromSweep :type Boolean) (SweepResult :type Hit%20Result%20Structure%20%28by%20ref%29))
  (Utilities|Casting|CastToBP_FallGuyCharacter OtherActor)
  (bind _asbp_fall_guy_game_mode (Utilities|Casting|CastToBP_FallGuyGameMode (Game|GetGameMode)))
  (Default|PickedSpeedBoost _asbp_fall_guy_game_mode)
  (Components|DestroyComponent (Variables|Default|GetBox))
  (Components|DestroyComponent (Variables|Default|GetBP_Coin))
  (Utilities|FlowControl|Delay (Variables|Default|GetDuration))
  (Default|RemoveSpeedBoost _asbp_fall_guy_game_mode)
  (Actor|DestroyActor))

(fn ConstructionScript)